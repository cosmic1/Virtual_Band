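; BP_FadableActor is a base actor for the DarkMatterXr content that tracks a fade value, starting at zero and inactive.
; SetTargetFadeValue and ToggleTargetFade set the target, and Tick moves the current value toward it at a constant FadeSpeed through UpdateFade, which reports whether it changed.
; Activate is an empty hook, called to switch on when a fade-in leaves zero and off when the fade returns to zero.
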(event EventTick
  (params (DeltaSeconds :type Float%20%28single-precision%29))
  (CallFunction|UpdateFade DeltaSeconds))

(event EventBeginPlay
  (bind _output_get (Variables|Default|SetFadeTarget 0.0))
  (Variables|Default|SetFade _output_get)
  (CallFunction|Activate false))

(fn ConstructionScript)

(fn SetTargetFadeValue
  (params (Fade :type Float%20%28single-precision%29))
  (bind _output_get (Variables|Default|SetFadeTarget Fade))
  (if (and (!= _output_get 0.0) (== (Variables|Default|GetFade) 0.0))
    (CallFunction|Activate true)))

(fn Activate
  (params (bActivate :type Boolean)))

(fn UpdateFade
  (params (DeltaTime :type Float%20%28single-precision%29))
  (if (!= (Variables|Default|GetFade) (Variables|Default|GetFadeTarget))
    (bind _output_get (Variables|Default|SetFade (Math|Interpolation|FInterptoConstant (Variables|Default|GetFade) (Variables|Default|GetFadeTarget) DeltaTime (Variables|Default|GetFadeSpeed))))
    (if (== _output_get 0.0)
      (CallFunction|Activate false))
    (return true)
    (else
      (return false))))

(fn ToggleTargetFade
  (if (> (Variables|Default|GetFadeTarget) 0.5)
    (CallFunction|SetTargetFadeValue 0.0)
    (else
      (CallFunction|SetTargetFadeValue 1.0))))