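; Fadable actor Blueprint for Niagara particle effects, extending its parent's fade and activation logic.
; When the parent fade update returns true, Fade is remapped into FadeRange and written to a named float parameter on every Niagara component.
; Activation shows the root hierarchy immediately.
; Deactivation sets a flag that Tick consumes, waiting the maximum particle lifetime and then hiding the hierarchy if Fade is zero.
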(event EventBeginPlay)

(event Collision|EventActorBeginOverlap
  (params (OtherActor :type Actor%20Object%20Reference)))

(event EventTick
  (params (DeltaSeconds :type Float%20%28single-precision%29))
  (|CallParentFunction DeltaSeconds)
  (if (Variables|Default|GetbStartDeactivation)
    (Variables|Default|SetbStartDeactivation false)
    (Utilities|FlowControl|Delay (Variables|Default|GetMaxParticleLifeTime))
    (if (== (Variables|Default|GetFade) 0.0)
      (Rendering|SetVisibility (Variables|Default|GetDefaultSceneRoot) false true))))

(fn ConstructionScript
  (|CallParentFunction))

(fn UpdateFadingParticles
  (bind _faderange (Variables|Default|GetFadeRange))
  (for _array_element (Actor|GetComponentsByClass "/Script/Niagara.NiagaraComponent")
    (Effects|Components|ParticleSystem|SetFloatParameter _array_element (Variables|Default|GetParticleFadeParameterName) (Math|Float|MapRangeClamped (Variables|Default|GetFade) 0.0 1.0 (.x _faderange) (.y _faderange)))))

(fn UpdateFade
  (params (DeltaTime :type Float%20%28single-precision%29))
  (bind _bupdated (|CallParentFunction DeltaTime))
  (if _bupdated
    (CallFunction|UpdateFadingParticles))
  (return _bupdated))

(fn Activate
  (params (bActivate :type Boolean))
  (|CallParentFunction bActivate)
  (if bActivate
    (Rendering|SetVisibility (Variables|Default|GetDefaultSceneRoot) true true)
    (else
      (Variables|Default|SetbStartDeactivation true))))